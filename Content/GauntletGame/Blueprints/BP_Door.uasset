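; BP_Door is a gauntlet game door that swings open when Activate is called.
; Exit doors show a closed material at BeginPlay and switch to an opened material on activation.
; A timeline lerps the mesh's relative rotation from its current value to a fixed absolute target.
; An exit door without a valid opened material never swings; the OpenDoor function and construction script are empty.
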(event EventBeginPlay
  (if (Variables|Exit|GetIsExitDoor)
    (bind _closed_material (Variables|Exit|GetClosed_Material)
      (:then
        (Rendering|Material|SetMaterial (Variables|Default|GetDoorMesh) 0 _closed_material))
      (:else))))

(event EventActivate
  (if (Variables|Exit|GetIsExitDoor)
    (bind _opened_material (Variables|Exit|GetOpened_Material)
      (:then
        (Rendering|Material|SetMaterial (Variables|Default|GetDoorMesh) 0 _opened_material))
      (:else)))
  (Variables|Default|SetInitial%20Rot (Variables|/Script/Engine.SceneComponent|GetRelativeRotation (Variables|Default|GetDoorMesh)))
  (bind _newtrack_0 (Timeline|OpeningAnimation Play)
    (:Update
      (Transformation|SetRelativeRotation (Variables|Default|GetDoorMesh) (Math|Rotator|Lerp(Rotator) (Variables|Default|GetInitial%20Rot) "0.000000,-90.000000,0.000000" _newtrack_0) false false))))

(fn ConstructionScript)

(fn OpenDoor)