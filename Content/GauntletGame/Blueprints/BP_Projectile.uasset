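; BP_Projectile is a reusable projectile that starts hidden and inactive, and is toggled on and off instead of spawned and destroyed.
; Activate places it at a given transform, shows it, enables collision and starts a lifetime timer.
; While active, Tick moves it along its forward vector with a swept SetActorLocation.
; Deactivate hides it, disables collision and parks it at a fixed off-field location.
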(event Collision|EventActorBeginOverlap
  (params (OtherActor :type Actor%20Object%20Reference)))

(event EventTick
  (params (DeltaSeconds :type Float%20%28single-precision%29))
  ;[0.15 0.15 0.15 0.5] TICK MOVEMENT
  (if (Variables|Default|GetIs%20Active)
    (Transformation|SetActorLocation (+ (Transformation|GetActorLocation) (* (* DeltaSeconds (Variables|Default|GetSpeed)) (Transformation|GetActorForwardVector))) true false)))

(event EventActivate
  (params (TransformData :type Transform))
  ;[0.15 0.15 0.15 0.5] ACTIVATE + LIFE TIMER
  (Rendering|SetActorHiddenInGame false)
  (Transformation|SetActorTransform TransformData)
  (Variables|Default|SetIs%20Active true)
  (Utilities|Time|SetTimerbyEvent (EventDispatchers|CreateEvent :!event BPDeactivate) (Variables|Default|GetActive%20Time))
  (Collision|SetActorEnableCollision true))

(event EventBeginPlay
  (Rendering|SetActorHiddenInGame true)
  (Variables|Default|SetIs%20Active false))

(event EventDeactivate
  ;[0.15 0.15 0.15 0.5] DEACTIVATE
  (Variables|Default|SetIs%20Active false)
  (Rendering|SetActorHiddenInGame true)
  (Collision|SetActorEnableCollision false)
  (Transformation|SetActorLocation "-1000.000000,-1000.000000,-1000.000000" false false))

(fn ConstructionScript)