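; BP_Turrett is a turret that continuously fires pooled BP_Projectile actors from its muzzle.
; BeginPlay fills the projectile pool and enables Tick, which takes a projectile from the pool every frame and activates it at the Muzzle's world transform.
; Activate and Deactivate work inversely to their names: Activate disables the turret by stopping Tick, Deactivate re-enables it, and each swaps the mesh material to match.
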(event EventBeginPlay
  (CallFunction|AddtoPool "/Game/GauntletGame/Blueprints/BP_Projectile.BP_Projectile_C" 20)
  (Actor|Tick|SetActorTickEnabled true))

(event EventTick
  (params (DeltaSeconds :type Float%20%28single-precision%29))
  (bind _poolable_actor (CallFunction|GetActorfromPool "/Game/GauntletGame/Blueprints/BP_Projectile.BP_Projectile_C"))
  (Class|Poolable|Activate _poolable_actor (Transformation|GetWorldTransform (Variables|Default|GetMuzzle))))

(event EventActivate
  ;[0.15 0.15 0.15 0.5] Turret Disabled
  (Actor|Tick|SetActorTickEnabled false)
  (Rendering|Material|SetMaterial (Variables|Default|GetMesh) 0 (Variables|Default|GetDeActivation%20Material)))

(event EventDeactivate
  ;[0.15 0.15 0.15 0.5] Turret Enabled
  (Actor|Tick|SetActorTickEnabled true)
  (Rendering|Material|SetMaterial (Variables|Default|GetMesh) 0 (Variables|Default|GetActivation%20Material)))

(fn ConstructionScript)