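; BP_Altar is an interactable altar that receives the artifact the main character carries on their back.
; On Interact, it detaches the item in BP_MainCharacter's back socket and moves it to the altar's Socket location.
; It then updates the quest through the quest subsystem and calls Activate on a linked ActorToControl via interface, which opens up the level exit.
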(event EventBeginPlay)

(event Collision|EventActorBeginOverlap
  (params (OtherActor :type Actor%20Object%20Reference)))

(event EventTick
  (params (DeltaSeconds :type Float%20%28single-precision%29)))

(event EventInteract
  (params (Interactor :type Actor%20Object%20Reference))
  (bind _actortocontrol (Variables|ControlledActor|GetActorToControl))
  ;[0.15 0.15 0.15 0.5] Detach the artifact and put it on new socket
  (bind _asbp_main_character (Utilities|Casting|CastToBP_MainCharacter Interactor))
  (bind _equipped_on_backsocket (Variables|/Game/GauntletGame/Character/BP_MainCharacter.BP_MainCharacter_C|GetEquipped%20On%20BackSocket _asbp_main_character)
    (:then
      (Transformation|DetachFromActor _equipped_on_backsocket "KeepRelative" "KeepRelative" "KeepRelative")
      (Transformation|SetActorLocation _equipped_on_backsocket (Transformation|GetWorldLocation (Variables|Default|GetSocket)) false false)
      ;[0.15 0.1315 0.03435 0.5] Update Quest and activate the exit
      (Class|QuestSubSystem|UpdateQuest (Subsystems|GetQuestSubSystem))
      (if (Utilities|IsValidInterface _actortocontrol)
        (Class|Activable|Activate _actortocontrol)))
    (:else)))

(fn ConstructionScript)